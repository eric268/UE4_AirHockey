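; Player paddle actor, driven by the mouse, for a puck-and-board game.
; Each tick, when the cursor trace does not hit a bp_board, it sweeps to the hit XY at a fixed height.
; It derives velocity from the position delta scaled by a fixed 60 rather than delta time.
; BeginPlay pauses the game, showing the cursor and BeginGame widget; overlapping a bp_Puck stores its reference.
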(event `self.ReceiveTick`
  (params (DeltaSeconds :type "Float (single-precision)"))
  (bind (_bblockinghit _binitialoverlap _time _distance _location _impactpoint _normal _impactnormal _physmat _hitactor) (`GameplayStatics.BreakHitResult` (`PlayerController.GetHitResultUnderCursorByChannel` (`GameplayStatics.GetPlayerController` 0) "TraceTypeQuery1" true)))
  ;[1 1 1] Links mos position  to paddle. Calculates veloctiy
  (set `self.CurrentPos` (`self.K2_GetActorLocation`))
  (cast `/Game/Blueprints/bp_board` _hitactor
    (:`CastFailed`
      (`self.K2_SetActorLocation` (`KismetMathLibrary.MakeVector` (.x _location) (.y _location) 26.0) true)
      (set `self.velocity` (* (- (`self.CurrentPos`) (`self.PrevPos`)) 60))
      (set `self.PrevPos` (`self.CurrentPos`)))))

(event `self.ReceiveBeginPlay`
  (`GameplayStatics.SetGamePaused` true)
  (set `PlayerController.bShowMouseCursor` true (`GameplayStatics.GetPlayerController` 0))
  (bind _returnvalue (`|CreateWidget` "/Game/UI/BeginGame.BeginGame_C"))
  (`UserWidget.AddToViewport` _returnvalue 0))

(event `self.ReceiveActorBeginOverlap`
  (params (OtherActor :type "Actor Object Reference"))
  (bind _asbp_puck (cast `/Game/Blueprints/bp_Puck` OtherActor))
  (set `self.Puck Ref` _asbp_puck))

(fn `UserConstructionScript`)