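; Puck actor for an air-hockey-style game, driven by collisions with paddles and goals.
; A hit from a paddle adds that paddle's velocity to the puck as a velocity-change impulse.
; Overlapping a paddle clears JustSpawned and teleports the puck slightly in X and Y to move it off the paddle.
; Two goal collision events cast the other actor and only store references to each goal.
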(event `self.ReceiveTick`
  (params (DeltaSeconds :type "Float (single-precision)")))

(event `Goal1 Collision`
  (params (OtherActor :type "Actor Object Reference"))
  (bind _asbp_goal (cast `/Game/Blueprints/bp_Goal` OtherActor))
  (set `self.Goal1 Ref` _asbp_goal))

(event `Goal 2 Collision`
  (params (OtherActor :type "Actor Object Reference"))
  (bind _asbp_goal_2 (cast `/Game/Blueprints/bp_Goal2` OtherActor))
  (set `self.Goal2 Ref` _asbp_goal_2))

(event `self.ReceiveActorBeginOverlap`
  (params (OtherActor :type "Actor Object Reference"))
  (bind (_returnvalue_x _returnvalue_y _returnvalue_z) (`KismetMathLibrary.BreakVector` (`self.K2_GetActorLocation`)))
  ;[1 1 1] Offsets puck if on top of paddle
  (cast `/Game/Blueprints/bp_Paddle` OtherActor)
  (if true
    (set `self.just spawned` false)
    (`self.K2_SetActorLocation` (`KismetMathLibrary.MakeVector` (+ _returnvalue_x 8.0) (+ _returnvalue_y 8.0) _returnvalue_z) false true)))

(event `self.ReceiveHit`
  (params (MyComp :type "PrimitiveComponent Object Reference") (Other :type "Actor Object Reference") (OtherComp :type "PrimitiveComponent Object Reference") (bSelfMoved :type Boolean) (HitLocation :type "Vector Structure") (HitNormal :type "Vector Structure") (NormalImpulse :type "Vector Structure") (Hit :type "HitResult Structure (by ref)"))
  ;[1 1 1] Transfers velocity from paddle to puck
  (bind _asbp_paddle (cast `/Game/Blueprints/bp_Paddle` Other))
  (`PrimitiveComponent.AddImpulse` (`self.puck`) (`/Game/Blueprints/bp_Paddle.velocity` _asbp_paddle) "None" true))

(fn `UserConstructionScript`)